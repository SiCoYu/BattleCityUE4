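; Player tank Blueprint, extending a base tank with lives, upgrade levels, score and kill counts held in PlayerData.
; Each level applies a style from the game instance; surviving a hit drops a level above one, and death resets it to zero.
; After death it either spends a life to respawn at its start location or notifies that the player is dead.
; Finishing spawning grants timed invincibility, shown by a cover sprite.
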(event Custom|StartInvincible
  (params (Interval :type Float%20%28single-precision%29))
  (bind _spritecover (Variables|Default|GetSpriteCover))
  (Variables|Game|SetbInvincible true)
  (Rendering|SetVisibility _spritecover true false)
  (Components|Timeline|PlayfromStart _spritecover)
  (Utilities|Time|SetTimerbyEvent (delegate Custom|StopInvincible) Interval))

(event Custom|StopInvincible
  (bind _spritecover (Variables|Default|GetSpriteCover))
  (Variables|Game|SetbInvincible false)
  (Audio|Components|Audio|Stop _spritecover)
  (Rendering|SetVisibility _spritecover false false))

(event EventBeginPlay
  (Game|SetLevel (Utilities|Struct|BreakS_Player (Variables|Config|GetPlayerData)))
  (Audio|Components|Audio|Stop (Variables|Default|GetSpriteCover))
  (Variables|Game|SetStartLocation (Transformation|GetActorLocation))
  (|CallParentFunction))

(event EventDead
  (CallFunction|SetState "NewEnumerator5")
  (|CallParentFunction)
  (if (>= (Utilities|Struct|BreakS_Player (Variables|Config|GetPlayerData)) 1)
    (Utilities|FlowControl|Delay 1.0)
    (Game|DecTank)
    (else
      (Default|CallNotifyPlayerDead (Variables|Config|GetPlayerIndex)))))

(event Game|Damage|EventAnyDamage
  (params (Damage :type Float%20%28single-precision%29) (DamageType :type Damage%20Type%20Object%20Reference) (InstigatedBy :type Controller%20Object%20Reference) (DamageCauser :type Actor%20Object%20Reference))
  (bind _playerdata (Variables|Config|GetPlayerData))
  (bind _level (Utilities|Struct|BreakS_Player _playerdata))
  (|CallParentFunction Damage DamageType InstigatedBy DamageCauser)
  (if (and (> (Variables|Default|GetHealth) 0.0) (> _level 1))
    (Game|SetLevel (- _level 1))
    (bind _state (CallFunction|GetState))
    (CallFunction|SetStateAnim (Math|Conversions|ToInteger(Byte) _state))
    (Audio|PlaySound2D "/Game/Assets/Audio/bullet_hit_1.bullet_hit_1" 1.0 1.0 0.0 0 0)))

(event EventDestroyed)

(fn ConstructionScript
  (|CallParentFunction))

(fn GetAnimStart
  (return (* (Variables|Config|GetPlayerIndex) 2)))

(fn CanApplyDamage
  (bind _value (|CallParentFunction))
  (return (and _value (not (Variables|Game|GetbInvincible)))))

(fn OnStateChange
  (params (Old :type E_State%20Enum :default "NewEnumerator0") (New :type E_State%20Enum :default "NewEnumerator0"))
  (|CallParentFunction Old New)
  (switch Utilities|FlowControl|Switch|SwitchonE_State New
    (:NewEnumerator5
      (Game|SetDeath))))

(fn OnStateFinished
  (bind _state (CallFunction|GetState))
  (switch Utilities|FlowControl|Switch|SwitchonE_State _state
    (:NewEnumerator0
      _)
    (:NewEnumerator1
      _)
    (:NewEnumerator3
      (CallFunction|StartInvincible 2.25))
    (:NewEnumerator4
      _)
    (:NewEnumerator5
      _))
  (|CallParentFunction))

(fn SetLevel
  (params (Level :type Integer))
  (Utilities|Struct|SetmembersinS_Player (Variables|Config|GetPlayerData) Level)
  (CallFunction|SetData (Utilities|Array|Get(acopy) (Variables|/Game/Blueprints/BP_GameInstance.BP_GameInstance_C|GetPlayerStyles (CallFunction|GetGameInstanceBP)) Level)))

(fn SetDeath
  (Rendering|SetVisibility (Variables|Default|GetSprite) false false)
  (Collision|SetCollisionEnabled (Variables|Default|GetBox) "NoCollision")
  (Default|Rotateto (Variables|Default|GetMovement) "NewEnumerator0")
  (Game|SetLevel)
  (CallFunction|SetStateAnim))

(fn Respawn
  (Transformation|SetActorLocation (Variables|Game|GetStartLocation) false true)
  (Rendering|SetVisibility (Variables|Default|GetSprite) true false)
  (Collision|SetCollisionEnabled (Variables|Default|GetBox) "QueryAndPhysics")
  (CallFunction|SetState "NewEnumerator3"))

(fn Levelup
  (Game|SetLevel (Math|Integer|Min(Integer) (+ (.Level (Utilities|Struct|BreakS_Player (Variables|Config|GetPlayerData))) 1) 3))
  (bind _state (CallFunction|GetState))
  (CallFunction|SetStateAnim (Math|Conversions|ToInteger(Byte) _state)))

(fn IncTank
  (params (Life :type Integer))
  (bind _playerdata (Variables|Config|GetPlayerData))
  (bind _life (Utilities|Struct|BreakS_Player _playerdata))
  (bind _returnvalue (+ Life _life))
  (Utilities|Struct|SetmembersinS_Player _playerdata _returnvalue)
  (Default|CallNotiyLifeChange (Variables|Config|GetPlayerIndex) _returnvalue))

(fn AddScore
  (params (Score :type Integer))
  (bind _playerdata (Variables|Config|GetPlayerData))
  (bind _score (Utilities|Struct|BreakS_Player _playerdata))
  (bind _returnvalue (+ Score _score))
  (Utilities|Struct|SetmembersinS_Player _playerdata _returnvalue)
  (Default|CallNotifyScoreChange (Variables|Config|GetPlayerIndex) _returnvalue))

(fn AddKillCount
  (params (Type :type Integer))
  (bind _playerdata (Variables|Config|GetPlayerData))
  (bind _killcount (Utilities|Struct|BreakS_Player _playerdata))
  (bind _result (Math|Integer|IncrementInt (Utilities|Array|Get(acopy) _killcount Type))
    (:%20%20
      (Utilities|Array|SetArrayElem _killcount Type _result))))

(fn DecTank
  (bind _playerdata (Variables|Config|GetPlayerData))
  (Utilities|Struct|SetmembersinS_Player _playerdata (- (Utilities|Struct|BreakS_Player _playerdata) 1))
  (Default|CallNotiyLifeChange (Variables|Config|GetPlayerIndex) (Utilities|Struct|BreakS_Player (Variables|Config|GetPlayerData)))
  (Game|Respawn))