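; BP_GameMode is a Game Mode Blueprint that handles flow between the main menu, level select, level editor and gameplay maps.
; Its events write session state to the game instance, such as player-two choice, custom-level flag and current level, then open maps by name.
; StartLevel clears statistics before loading the shared Level map, or calls GameOver to return to the main menu when the requested level exceeds MaxLevel.
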(event Custom|GameOver
  (Game|OpenLevel(byName) "MainMenu"))

(event Custom|MainMenu
  (Game|OpenLevel(byName) "MainMenu"))

(event Custom|StartGame
  (params (PlayerTwo :type Boolean))
  (bind _newparam (CallFunction|GetGameInstanceBP))
  (Variables|/Game/Blueprints/BP_GameInstance.BP_GameInstance_C|SetPlayerTwo _newparam PlayerTwo)
  (Default|InitData _newparam)
  (Game|OpenLevel(byName) "SelectLevel"))

(event Custom|StartEdit
  (Variables|/Game/Blueprints/BP_GameInstance.BP_GameInstance_C|SetCustomLevel (CallFunction|GetGameInstanceBP) true)
  (Game|OpenLevel(byName) "Editor"))

(event Custom|StartLevel
  (params (Level :type Integer))
  (bind _newparam (CallFunction|GetGameInstanceBP))
  (if (<= Level (Variables|/Game/Blueprints/BP_GameInstance.BP_GameInstance_C|GetMaxLevel _newparam))
    (Variables|/Game/Blueprints/BP_GameInstance.BP_GameInstance_C|SetCurrentLevel _newparam Level)
    (Default|ClearStatistics (CallFunction|GetGameInstanceBP))
    (Game|OpenLevel(byName) "Level")
    (else
      (CallFunction|GameOver))))

(fn ConstructionScript)