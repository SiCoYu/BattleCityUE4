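; AI controller for enemy tanks that drives random movement and periodic shooting of the possessed BP_Tank.
; Possession starts a looping shoot timer and a one-shot MakeChoice timer, and UnPossess clears both.
; MakeChoice picks a weighted random direction based on tile X versus a center column, but its re-arm timer misspells the function as "MakeCoice".
; Hits randomly trigger a new choice or a brief stop through Think.
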(event Custom|OnHit
  (params (SelfActor :type Actor%20Object%20Reference) (OtherActor :type Actor%20Object%20Reference) (NormalImpulse :type Vector) (Hit :type Hit%20Result%20Structure%20%28by%20ref%29))
  (switch int (Math|Random|RandomInteger 4)
    (:0
      (CallFunction|MakeChoice :!label _label))
    (:1
      (CallFunction|Think 1.0 :!label _label_2))
    (:2
      (goto _label))
    (:3
      (goto _label_2))))

(event Custom|StartShoot
  (bind _target (Variables|Game|GetTarget))
  (Utilities|IsValid _target
    (:Is%20Valid
      (Default|Shoot _target))))

(event EventUnPossess
  (params (UnpossessedPawn :type Pawn%20Object%20Reference))
  (Utilities|Time|ClearandInvalidateTimerbyHandle (Variables|Game|GetTimerShoot))
  (Utilities|Time|ClearandInvalidateTimerbyHandle (Variables|Game|GetTimerMakeChoise)))

(event EventPossess
  (params (PossessedPawn :type Pawn%20Object%20Reference))
  (bind _asbp_tank (Utilities|Casting|CastToBP_Tank PossessedPawn))
  (bind _output_get (Variables|Game|SetTarget _asbp_tank))
  (Collision|BindEventtoOnActorHit _output_get (delegate Custom|OnHit))
  (bind _returnvalue (Utilities|Time|SetTimerbyFunctionName self "MakeChoice" (Variables|Config|GetThinkTime)))
  (Variables|Game|SetTimerMakeChoise _returnvalue)
  (bind _returnvalue_2 (Utilities|Time|SetTimerbyEvent (delegate Custom|StartShoot) (Variables|Config|GetShootInterval) true))
  (Variables|Game|SetTimerShoot _returnvalue_2))

(fn ConstructionScript)

(fn Think
  (params (Interval :type Float%20%28single-precision%29))
  (bind _target (Variables|Game|GetTarget))
  (bind _movement (Variables|/Game/Blueprints/Tank/BP_Tank.BP_Tank_C|GetMovement _target))
  (Default|Stopby _movement (Variables|/Game/Blueprints/Tank/Component/BP_Movement.BP_Movement_C|GetDirection _movement))
  (bind _returnvalue (Utilities|Time|SetTimerbyFunctionName self "MakeChoice" Interval))
  (Variables|Game|SetTimerMakeChoise _returnvalue))

(fn MakeChoice
  (bind _returnvalue (Math|Random|RandomInteger 6))
  (bind _target (Variables|Game|GetTarget))
  (bind _movement (Variables|/Game/Blueprints/Tank/BP_Tank.BP_Tank_C|GetMovement _target))
  (Utilities|FlowControl|Sequence
    (:then_0
      (bind _output_get (Variables|Config|SetThinkTime (Math|Random|RandomFloatinRange 3.0 4.0)))
      (bind _returnvalue_2 (Utilities|Time|SetTimerbyFunctionName self "MakeCoice" _output_get))
      (Variables|Game|SetTimerMakeChoise _returnvalue_2))
    (:then_1
      (Math|Integer|CompareInt (Math|Float|Truncate (.x (CallFunction|GetTileIndex (Transformation|GetActorLocation (Variables|Game|GetTarget))))) 7
        (:>
          (Default|Moveby _movement (Utilities|Select :Index _returnvalue :Option%200 "NewEnumerator2" :Option%201 "NewEnumerator1" :Option%202 "NewEnumerator3" :Option%203 "NewEnumerator0" :Option%204 "NewEnumerator3" :Option%205 "NewEnumerator2")))
        (:==
          (Default|Moveby _movement (Utilities|Select :Index _returnvalue :Option%200 "NewEnumerator2" :Option%201 "NewEnumerator1" :Option%202 "NewEnumerator3" :Option%203 "NewEnumerator0" :Option%204 "NewEnumerator0" :Option%205 "NewEnumerator0")))
        (:<
          (Default|Moveby _movement (Utilities|Select :Index _returnvalue :Option%200 "NewEnumerator2" :Option%201 "NewEnumerator1" :Option%202 "NewEnumerator3" :Option%203 "NewEnumerator0" :Option%204 "NewEnumerator1" :Option%205 "NewEnumerator2")))))))