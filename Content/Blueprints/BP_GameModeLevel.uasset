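; Game mode for a tank battle level that runs one or two players against a queue of enemies.
; On BeginPlay it builds the HUD, spawns players at BP_Level locations and spawns enemies on a looping timer.
; Bound kill events award score and trigger item drops through ItemManager.
; Clearing all enemies saves player data and opens LevelStatistics, while losing all players shows game over, then returns to MainMenu.
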(event Custom|GameOver
  (bind _returnvalue (UserInterface|CreateWidget "/Game/Assets/UI/WB_GameOver.WB_GameOver_C"))
  (UserInterface|Viewport|AddtoViewport _returnvalue 0)
  (Input|SetInputModeUIOnly (Game|GetPlayerController 0) _returnvalue "DoNotLock")
  (EventDispatchers|BindEventtoNotifyGameOver _returnvalue (delegate Custom|EndLevel))
  (Utilities|Time|ClearandInvalidateTimerbyHandle (Variables|Game|GetEnemyTimer))
  (bind _outactors (Actor|GetAllActorsOfClass "/Game/Blueprints/Tank/Enemy/BP_EnemyController.BP_EnemyController_C"))
  (for _array_element _outactors
    (Pawn|UnPossess _array_element)))

(event Custom|CheckFinished
  (if (and (== (Utilities|Array|Length (Variables|/Game/Blueprints/BP_GameInstance.BP_GameInstance_C|GetEnemies (CallFunction|GetGameInstanceBP))) 0) (== (Variables|Game|GetEnemyCount) 0))
    (CallFunction|SavePlayerData)
    (Utilities|FlowControl|Delay 2.0)
    (Game|OpenLevel(byName) "LevelStatistics")))

(event Custom|EndLevel
  (Game|OpenLevel(byName) "MainMenu"))

(event EventBeginPlay
  (Utilities|FlowControl|Sequence
    (:then_0
      (bind _outactors (Actor|GetAllActorsOfClass "/Game/Blueprints/Level/BP_Level.BP_Level_C"))
      (Variables|Game|SetLevel (Utilities|Array|Get(acopy) _outactors)))
    (:then_1
      (CallFunction|InitUI))
    (:then_2
      (CallFunction|StartSpawnPlayer))
    (:then_3
      (CallFunction|StartSpawnEnemy))))

(event Custom|StartSpawnEnemy
  (bind _returnvalue (Utilities|Time|SetTimerbyEvent (delegate Custom|SpawnEnemy) (Variables|Config|GetSpawnInterval) true))
  (Variables|Game|SetEnemyTimer _returnvalue))

(event Custom|SpawnEnemy
  (if (> (Default|GetEnemyLeftCount (CallFunction|GetGameInstanceBP)) 0)
    (bind _enemy (CallFunction|CreateEnemyTank))
    (CallFunction|BindEnemy _enemy)
    (Math|Integer|IncrementInt (Variables|Game|GetEnemyCount)
      (:%20%20
        (Default|DecreaseEnemy (Variables|Game|GetGameInfo))))))

(event Custom|BindEnemy
  (params (Enemy :type BP%20Enemy%20Object%20Reference))
  (EventDispatchers|BindEventtoNotifyKilled Enemy (delegate Custom|EnemyKilled))
  (Default|OnSpawnEnemy (Variables|Default|GetItemManager) Enemy))

(event Custom|EnemyKilled
  (params (Killer :type Actor%20Object%20Reference) (Target :type Actor%20Object%20Reference) (NewParam :type Boolean))
  (CallFunction|KillEnemy Killer Target true))

(event Custom|StartSpawnPlayer
  (CallFunction|CreatePlayerTank)
  (if (Variables|/Game/Blueprints/BP_GameInstance.BP_GameInstance_C|GetPlayerTwo (CallFunction|GetGameInstanceBP))
    (CallFunction|CreatePlayerTank 1)))

(event Custom|LIfeChange
  (params (Index :type Integer) (Life :type Integer))
  (CallFunction|UpdateLife Index Life))

(event Custom|PlayerDead
  (params (Index :type Integer))
  (bind _result (Math|Integer|IncrementInt (Variables|Game|GetDeadPlayer))
    (:%20%20
      (if (== _result (Utilities|Array|Length (Variables|Game|GetPlayer)))
        (CallFunction|GameOver)))))

(event Custom|ScoreChange
  (params (Index :type Integer) (Score :type Integer))
  (CallFunction|UpdateScore Index Score))

(event Custom|BindPlayer
  (params (Player :type BP%20Player%20Object%20Reference))
  (EventDispatchers|BindEventtoNotifyScoreChange Player (delegate Custom|ScoreChange))
  (EventDispatchers|BindEventtoNotiyLifeChange Player (delegate Custom|LIfeChange))
  (EventDispatchers|BindEventtoNotifyPlayerDead Player (delegate Custom|PlayerDead)))

(fn ConstructionScript)

(fn CreatePlayerTank
  (params (Index :type Integer))
  (bind _level (Variables|Game|GetLevel))
  (bind _playerlocations (Variables|/Game/Blueprints/Level/BP_Level.BP_Level_C|GetPlayerLocations _level))
  (bind _output (Utilities|Array|Get(acopy) _playerlocations Index))
  (bind _returnvalue (Game|SpawnActorfromClass "/Game/Blueprints/Tank/Player/BP_Player.BP_Player_C" (Math|Transform|MakeTransform (Math|Vector|MakeVector (.x _output) (.y _output) 0.0) "0, 0, 0" "1,1,1") "AlwaysSpawn" 0 (Utilities|Array|Get(acopy) (Variables|/Game/Blueprints/BP_GameInstance.BP_GameInstance_C|GetPlayerDatas (CallFunction|GetGameInstanceBP)) Index) Index 0))
  (bind _controller (CallFunction|GetPlayerControllerBP))
  (Default|Possess _controller Index _returnvalue)
  (Utilities|Array|Add (Variables|Game|GetPlayer) _returnvalue)
  (CallFunction|BindPlayer _returnvalue))

(fn CreateEnemyTank
  (bind _newparam (CallFunction|GetGameInstanceBP))
  (bind _level (Variables|Game|GetLevel))
  (bind _newparam_2 (Default|GetEnemyLeftCount _newparam))
  (bind _enemylocations (Variables|/Game/Blueprints/Level/BP_Level.BP_Level_C|GetEnemyLocations _level))
  (bind _returnvalue (Math|Integer|%(Integer) _newparam_2 3))
  (bind _output (Utilities|Array|Get(acopy) _enemylocations _returnvalue))
  (bind _returnvalue_2 (Game|SpawnActorfromClass "/Game/Blueprints/Tank/Enemy/BP_Enemy.BP_Enemy_C" (Math|Transform|MakeTransform (Math|Vector|MakeVector (.x _output) (.y _output) 0.0) "0, 0, 0" "1,1,1") "AlwaysSpawn" 0 (Default|AquireOneEnemy _newparam) (Default|EnemyHasItem _newparam) 0))
  (return _returnvalue_2))

(fn InitUI
  (bind _newparam (CallFunction|GetGameInstanceBP))
  (bind _returnvalue (UserInterface|CreateWidget "/Game/Assets/UI/WB_LevelInfo.WB_LevelInfo_C"))
  (bind _output_get (Variables|Game|SetGameInfo _returnvalue))
  (UserInterface|Viewport|AddtoViewport _output_get 0)
  (Default|SetStage _output_get (Variables|/Game/Blueprints/BP_GameInstance.BP_GameInstance_C|GetCurrentLevel _newparam))
  (Default|EnablePlayer2 _output_get (Variables|/Game/Blueprints/BP_GameInstance.BP_GameInstance_C|GetPlayerTwo _newparam))
  (for (_array_element _array_index) (Variables|/Game/Blueprints/BP_GameInstance.BP_GameInstance_C|GetPlayerDatas _newparam)
    (Default|SetLIfe _output_get _array_index (.Life (Utilities|Struct|BreakS_Player _array_element)))))

(fn SavePlayerData
  (for (_array_element _array_index) (Variables|Game|GetPlayer)
    (Utilities|Array|SetArrayElem (Variables|/Game/Blueprints/BP_GameInstance.BP_GameInstance_C|GetPlayerDatas (CallFunction|GetGameInstanceBP)) _array_index (Variables|/Game/Blueprints/Tank/Player/BP_Player.BP_Player_C|GetPlayerData _array_element))))

(fn UpdateScore
  (params (Player :type Integer) (Score :type Integer)))

(fn UpdateLife
  (params (Player :type Integer) (Life :type Integer))
  (Default|SetLIfe (Variables|Game|GetGameInfo) Player Life))

(fn KillEnemy
  (params (Killer :type Actor%20Object%20Reference) (Target :type Actor%20Object%20Reference) (Popup :type Boolean))
  (Utilities|FlowControl|Sequence
    (:then_0
      (bind _asbp_player (Utilities|Casting|CastToBP_Player Killer))
      (bind _asbp_enemy (Utilities|Casting|CastToBP_Enemy Target))
      (Default|AddScore _asbp_player (Utilities|Struct|BreakS_Tank (Variables|/Game/Blueprints/Tank/BP_Tank.BP_Tank_C|GetData _asbp_enemy)))
      (Default|AddKillCount _asbp_player (Variables|/Game/Blueprints/Tank/Enemy/BP_Enemy.BP_Enemy_C|GetType _asbp_enemy))
      (if Popup
        (Game|SpawnActorfromClass "/Game/Blueprints/Tank/Player/BP_Score.BP_Score_C" (Math|Transform|MakeTransform (- (Transformation|GetActorLocation _asbp_enemy) "16.000000,16.000000, 0") "0, 0, 0" "1,1,1") "Undefined" 0 (Utilities|Struct|BreakS_Tank (Variables|/Game/Blueprints/Tank/BP_Tank.BP_Tank_C|GetData _asbp_enemy)) 0)
        (if (Variables|/Game/Blueprints/Tank/Enemy/BP_Enemy.BP_Enemy_C|GetBonus _asbp_enemy)
          (Default|CreateItem (Variables|Default|GetItemManager)))))
    (:then_1
      (Math|Integer|DecrementInt (Variables|Game|GetEnemyCount)))
    (:then_2
      (CallFunction|CheckFinished))))