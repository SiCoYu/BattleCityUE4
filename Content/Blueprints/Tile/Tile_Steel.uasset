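; Steel tile actor that is destroyed only by a single hit of more than 1 damage.
; Its AnyDamage event ignores weaker hits and keeps no running health total.
; ToggleTile flips IsBrick and swaps the Tile sprite between brick and steel, while the damage check stays independent of that flag.
; The construction script only runs the parent's setup.
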(event Game|Damage|EventAnyDamage
  (params (Damage :type Float%20%28single-precision%29) (DamageType :type Damage%20Type%20Object%20Reference) (InstigatedBy :type Controller%20Object%20Reference) (DamageCauser :type Actor%20Object%20Reference))
  (if (> Damage 1.0)
    (Actor|DestroyActor)))

(fn ConstructionScript
  (|CallParentFunction))

(fn ToggleTile
  (bind _output_get (Variables|Default|SetIsBrick (not (Variables|Default|GetIsBrick))))
  (Rendering|Components|Sprite|SetSprite (Variables|Default|GetTile) (select _output_get "/Game/Assets/Sprites/Levels/BrickTile.BrickTile" "/Game/Assets/Sprites/Tile/SpriteSteel.SpriteSteel")))