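; BP_Slide is a tank component that makes its owner keep gliding for a short distance on ice.
; Each tick it reads the owner's state message; a change into the first state while OnIce is set starts a fixed-distance slide.
; While sliding, it drives the owner's BP_Movement and counts the distance down by movement speed.
; The slide ends when the distance runs out, the ice is left or the second state occurs.
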(event EventBeginPlay
  (bind _returnvalue (Components|GetOwner))
  (Variables|Default|SetTarget _returnvalue)
  (Variables|Default|SetMovement (Actor|GetComponentbyClass _returnvalue "/Game/Blueprints/Tank/Component/BP_Movement.BP_Movement_C")))

(event EventTick
  (params (DeltaSeconds :type Float%20%28single-precision%29))
  (bind _state (Class|IBState|GetState(Message) (Variables|Default|GetTarget)))
  (Utilities|FlowControl|Sequence
    (:then_0
      (CallFunction|StartSliding _state))
    (:then_1
      (CallFunction|ProcessSliding _state DeltaSeconds))))

(fn StartSliding
  (params (State :type E_State%20Enum :default "NewEnumerator0"))
  (if (Utilities|Enum|NotEqual(Enum) State (Variables|Default|GetState))
    (bind _output_get (Variables|Default|SetState State))
    (if (and (Utilities|Enum|Equal(Enum) _output_get "NewEnumerator0") (Variables|Default|GetbOnIce))
      (Variables|Default|SetbSliding true)
      (Variables|Default|SetDistanceToSlide 32.0))))

(fn ProcessSliding
  (params (State :type E_State%20Enum :default "NewEnumerator0") (Delta :type Float%20%28single-precision%29))
  (Utilities|FlowControl|Sequence
    (:then_0
      (if (Utilities|Enum|Equal(Enum) State "NewEnumerator1")
        (Variables|Default|SetbSliding false)
        (Variables|Default|SetDistanceToSlide 0.0)))
    (:then_1
      (if (not (Variables|Default|GetbOnIce))
        (Variables|Default|SetbSliding false)))
    (:then_2
      (if (Variables|Default|GetbSliding)
        (bind _output_get (Variables|Default|SetDistanceToSlide (Math|Float|Max(Float) (- (Variables|Default|GetDistanceToSlide) (* Delta (Variables|/Game/Blueprints/Tank/Component/BP_Movement.BP_Movement_C|GetSpeed (Variables|Default|GetMovement)))) 0.0)))
        (Default|MoveTarget (Variables|Default|GetMovement) Delta)
        (if (<= _output_get 0.0)
          (Variables|Default|SetbSliding false))))))