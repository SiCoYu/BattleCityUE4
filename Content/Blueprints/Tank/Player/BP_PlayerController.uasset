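; Player controller that drives two tanks for local two-player play from a single controller.
; Possess stores a tank in the Tanks array by index instead of using engine possession, and each player's input actions target their own slot.
; Direction presses and releases start and stop the tank's Movement component in one of four directions, while both A and B buttons fire its Shoot, all guarded by validity checks.
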(event Input|ActionEvents|InputActionA_2
  (params (Key :type Key%20Structure :default "None"))
  (bind _tanks (Variables|Game|GetTanks))
  (bind _output (Utilities|Array|Get(acopy) _tanks 1))
  (:Pressed
    (Utilities|IsValid _output
      (:Is%20Valid
        (Default|Shoot _output)))))

(event Input|ActionEvents|InputActionB_2
  (params (Key :type Key%20Structure :default "None"))
  (bind _tanks (Variables|Game|GetTanks))
  (bind _output (Utilities|Array|Get(acopy) _tanks 1))
  (:Pressed
    (Utilities|IsValid _output
      (:Is%20Valid
        (Default|Shoot _output)))))

(event Input|ActionEvents|InputActionUp_1
  (params (Key :type Key%20Structure :default "None"))
  (bind _tanks (Variables|Game|GetTanks))
  (bind _output (Utilities|Array|Get(acopy) _tanks))
  (bind _movement (Variables|/Game/Blueprints/Tank/BP_Tank.BP_Tank_C|GetMovement _output))
  (:Pressed
    (Utilities|IsValid _output
      (:Is%20Valid
        (Default|Moveby _movement "NewEnumerator0"))))
  (:Released
    (Utilities|IsValid _output
      (:Is%20Valid
        (Default|Stopby _movement "NewEnumerator0")))))

(event Input|ActionEvents|InputActionRight_1
  (params (Key :type Key%20Structure :default "None"))
  (bind _tanks (Variables|Game|GetTanks))
  (bind _output (Utilities|Array|Get(acopy) _tanks))
  (bind _movement (Variables|/Game/Blueprints/Tank/BP_Tank.BP_Tank_C|GetMovement _output))
  (:Pressed
    (Utilities|IsValid _output
      (:Is%20Valid
        (Default|Moveby _movement "NewEnumerator1"))))
  (:Released
    (Utilities|IsValid _output
      (:Is%20Valid
        (Default|Stopby _movement "NewEnumerator1")))))

(event Input|ActionEvents|InputActionDown_1
  (params (Key :type Key%20Structure :default "None"))
  (bind _tanks (Variables|Game|GetTanks))
  (bind _output (Utilities|Array|Get(acopy) _tanks))
  (bind _movement (Variables|/Game/Blueprints/Tank/BP_Tank.BP_Tank_C|GetMovement _output))
  (:Pressed
    (Utilities|IsValid _output
      (:Is%20Valid
        (Default|Moveby _movement "NewEnumerator2"))))
  (:Released
    (Utilities|IsValid _output
      (:Is%20Valid
        (Default|Stopby _movement "NewEnumerator2")))))

(event Input|ActionEvents|InputActionLeft_1
  (params (Key :type Key%20Structure :default "None"))
  (bind _tanks (Variables|Game|GetTanks))
  (bind _output (Utilities|Array|Get(acopy) _tanks))
  (bind _movement (Variables|/Game/Blueprints/Tank/BP_Tank.BP_Tank_C|GetMovement _output))
  (:Pressed
    (Utilities|IsValid _output
      (:Is%20Valid
        (Default|Moveby _movement "NewEnumerator3"))))
  (:Released
    (Utilities|IsValid _output
      (:Is%20Valid
        (Default|Stopby _movement "NewEnumerator3")))))

(event Input|ActionEvents|InputActionUp_2
  (params (Key :type Key%20Structure :default "None"))
  (bind _tanks (Variables|Game|GetTanks))
  (bind _output (Utilities|Array|Get(acopy) _tanks 1))
  (bind _movement (Variables|/Game/Blueprints/Tank/BP_Tank.BP_Tank_C|GetMovement _output))
  (:Pressed
    (Utilities|IsValid _output
      (:Is%20Valid
        (Default|Moveby _movement "NewEnumerator0"))))
  (:Released
    (Utilities|IsValid _output
      (:Is%20Valid
        (Default|Stopby _movement "NewEnumerator0")))))

(event Input|ActionEvents|InputActionRight_2
  (params (Key :type Key%20Structure :default "None"))
  (bind _tanks (Variables|Game|GetTanks))
  (bind _output (Utilities|Array|Get(acopy) _tanks 1))
  (bind _movement (Variables|/Game/Blueprints/Tank/BP_Tank.BP_Tank_C|GetMovement _output))
  (:Pressed
    (Utilities|IsValid _output
      (:Is%20Valid
        (Default|Moveby _movement "NewEnumerator1"))))
  (:Released
    (Utilities|IsValid _output
      (:Is%20Valid
        (Default|Stopby _movement "NewEnumerator1")))))

(event Input|ActionEvents|InputActionDown_2
  (params (Key :type Key%20Structure :default "None"))
  (bind _tanks (Variables|Game|GetTanks))
  (bind _output (Utilities|Array|Get(acopy) _tanks 1))
  (bind _movement (Variables|/Game/Blueprints/Tank/BP_Tank.BP_Tank_C|GetMovement _output))
  (:Pressed
    (Utilities|IsValid _output
      (:Is%20Valid
        (Default|Moveby _movement "NewEnumerator2"))))
  (:Released
    (Utilities|IsValid _output
      (:Is%20Valid
        (Default|Stopby _movement "NewEnumerator2")))))

(event Input|ActionEvents|InputActionLeft_2
  (params (Key :type Key%20Structure :default "None"))
  (bind _tanks (Variables|Game|GetTanks))
  (bind _output (Utilities|Array|Get(acopy) _tanks 1))
  (bind _movement (Variables|/Game/Blueprints/Tank/BP_Tank.BP_Tank_C|GetMovement _output))
  (:Pressed
    (Utilities|IsValid _output
      (:Is%20Valid
        (Default|Moveby _movement "NewEnumerator3"))))
  (:Released
    (Utilities|IsValid _output
      (:Is%20Valid
        (Default|Stopby _movement "NewEnumerator3")))))

(event Input|ActionEvents|InputActionB_1
  (params (Key :type Key%20Structure :default "None"))
  (bind _tanks (Variables|Game|GetTanks))
  (bind _output (Utilities|Array|Get(acopy) _tanks))
  (:Pressed
    (Utilities|IsValid _output
      (:Is%20Valid
        (Default|Shoot _output)))))

(event Input|ActionEvents|InputActionA_1
  (params (Key :type Key%20Structure :default "None"))
  (bind _tanks (Variables|Game|GetTanks))
  (bind _output (Utilities|Array|Get(acopy) _tanks))
  (:Pressed
    (Utilities|IsValid _output
      (:Is%20Valid
        (Default|Shoot _output)))))

(fn ConstructionScript)

(fn Possess
  (params (Index :type Integer) (Tank :type BP%20Player%20Object%20Reference))
  (Utilities|Array|SetArrayElem (Variables|Game|GetTanks) Index Tank))