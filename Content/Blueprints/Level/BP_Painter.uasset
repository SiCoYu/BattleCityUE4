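; BP_Painter spawns a square grid of Tile actors, CellNum cells per side and TileWidth apart.
; The construction script sizes and offsets a Box to cover the grid, and BeginPlay fills it when Editor is set.
; CreateTiles spawns and returns tiles for an index range.
; Draw paints a full grid at a location snapped to 32 units, while Shift uses an index to pick the full grid or one half.
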(event EventBeginPlay
  (bind _cellnum (Variables|Config|GetCellNum))
  (bind _returnvalue (- _cellnum 1))
  (if (Variables|Config|GetEditor)
    (CallFunction|CreateTiles 0 _returnvalue 0 _returnvalue (Transformation|GetActorLocation))))

(fn ConstructionScript
  (bind _box (Variables|Default|GetBox))
  (bind _tilewidth (Variables|Config|GetTileWidth))
  (bind _cellnum (Variables|Config|GetCellNum))
  (bind _returnvalue (* _cellnum _tilewidth))
  (bind _returnvalue_2 (/ _returnvalue 2.0))
  (Components|Box|SetBoxExtent _box (Math|Vector|MakeVector _returnvalue_2 _returnvalue_2 8.0) true)
  (Transformation|SetRelativeLocation _box (Math|Vector|MakeVector _returnvalue_2 _returnvalue_2 0.0) false false))

(fn CreateTiles
  (params (FirstX :type Integer) (LastX :type Integer) (FirstY :type Integer) (LastY :type Integer) (Location :type Vector))
  (bind _tilewidth (Variables|Config|GetTileWidth))
  (for _index (range FirstX LastX)
    (for _index_2 (range FirstY LastY)
      (bind _returnvalue (Game|SpawnActorfromClass (Variables|Config|GetTile) (Math|Transform|MakeTransform (+ (Math|Vector|MakeVector (* _index _tilewidth) (* _index_2 _tilewidth) 0.0) Location) "0, 0, 0" "1,1,1") "AlwaysSpawn" 0 0))
      (Utilities|Array|Add (LocalVariables|GetTempList) _returnvalue)))
  (return (LocalVariables|GetTempList)))

(fn Shift
  (params (Location :type Vector) (Index :type Integer))
  (bind _returnvalue (/ Location 32.0))
  (bind _cellnum (Variables|Config|GetCellNum))
  (bind _returnvalue_2 (- _cellnum 1))
  (bind _returnvalue_3 (/ _cellnum 2))
  (bind _returnvalue_4 (- _returnvalue_3 1))
  (bind _list (CallFunction|CreateTiles (Utilities|Select :Index Index :Option%200 0 :Option%201 0 :Option%202 _returnvalue_3 :Option%203 0 :Option%204 0) (Utilities|Select :Index Index :Option%200 _returnvalue_2 :Option%201 _returnvalue_2 :Option%202 _returnvalue_2 :Option%203 _returnvalue_2 :Option%204 _returnvalue_4) (Utilities|Select :Index Index :Option%200 0 :Option%201 0 :Option%202 0 :Option%203 _returnvalue_3 :Option%204 0) (Utilities|Select :Index Index :Option%200 _returnvalue_2 :Option%201 _returnvalue_4 :Option%202 _returnvalue_2 :Option%203 _returnvalue_2 :Option%204 _returnvalue_2) (Math|Vector|MakeVector (* (Math|Float|Floor (.x _returnvalue)) 32.0) (* (Math|Float|Floor (.y _returnvalue)) 32.0) 0.0)))
  (return _list))

(fn Draw
  (params (Location :type Vector))
  (bind _returnvalue (/ Location 32.0))
  (bind _cellnum (Variables|Config|GetCellNum))
  (bind _returnvalue_2 (- _cellnum 1))
  (bind _list (CallFunction|CreateTiles 0 _returnvalue_2 0 _returnvalue_2 (Math|Vector|MakeVector (* (Math|Float|Floor (.x _returnvalue)) 32.0) (* (Math|Float|Floor (.y _returnvalue)) 32.0) 0.0)))
  (return _list))