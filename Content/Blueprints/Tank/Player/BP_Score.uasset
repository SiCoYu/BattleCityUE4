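; BP_Score is a short-lived actor that displays a score value through a widget component, likely as a score popup.
; Its SetScore function casts the component's user widget to WB_Score and passes the Score value to it.
; The construction script and BeginPlay both apply the score, then BeginPlay waits for the Delay variable's duration and destroys the actor.
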(event EventBeginPlay
  (CallFunction|SetScore (Variables|Config|GetScore))
  (Utilities|FlowControl|Delay (Variables|Config|GetDelay))
  (Actor|DestroyActor))

(event Collision|EventActorBeginOverlap
  (params (OtherActor :type Actor%20Object%20Reference)))

(event EventTick
  (params (DeltaSeconds :type Float%20%28single-precision%29)))

(fn ConstructionScript
  (CallFunction|SetScore (Variables|Config|GetScore)))

(fn SetScore
  (params (Score :type Integer))
  (bind _aswb_score (Utilities|Casting|CastToWB_Score (UserInterface|GetUserWidgetObject (Variables|Default|GetWidget))))
  (Default|SetScore _aswb_score Score))