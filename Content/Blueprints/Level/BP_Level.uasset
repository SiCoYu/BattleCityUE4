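; Level actor for a tile-based, Battle City-style game that spawns the eagle base and its brick surround, in either play or editor mode.
; LoadLevel reads a tile map from the game instance, then notifies the editor or stamps tiles through temporary painter actors on a 13-wide grid.
; The shovel power-up rebuilds the surround in steel, flickers it on a looping timer near expiry, then restores brick.
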(event Custom|StartShovel
  (CallFunction|CreateSurrounding true)
  (Utilities|Time|SetTimerbyEvent (delegate Custom|StartShovelFlicker) 18.0)
  (Utilities|Time|SetTimerbyEvent (delegate Custom|StopShovel) 21.0))

(event Custom|StartShovelFlicker
  (bind _returnvalue (Utilities|Time|SetTimerbyEvent (delegate Custom|ShovelFlicker) 0.28 true))
  (Variables|Game|SetShovelTimer _returnvalue))

(event Custom|StopShovel
  (CallFunction|CreateSurrounding false)
  (Utilities|Time|ClearandInvalidateTimerbyHandle (Variables|Game|GetShovelTimer)))

(event Custom|ShovelFlicker
  (for _array_element (Variables|Game|GetShovel)
    (Utilities|IsValid _array_element
      (:Is%20Valid
        (bind _astile_steel (Utilities|Casting|CastToTile_Steel _array_element))
        (Default|ToggleTile _astile_steel)))))

(event EventBeginPlay
  (if (Variables|Config|GetbEditor)
    (CallFunction|InitEditor)
    (else
      (CallFunction|InitGame)))
  (CallFunction|CreateEagle))

(fn ConstructionScript)

(fn InitGame
  (bind _returnvalue (Game|GetPlayerController 0))
  (Game|Player|SetViewTargetwithBlend _returnvalue self 0.0 "VTBlend_Linear" 0.0 false)
  (Variables|/Script/Engine.PlayerController|SetbShowMouseCursor _returnvalue false)
  (Variables|/Script/Engine.PlayerController|SetbEnableClickEvents _returnvalue false)
  (Input|SetInputModeGameOnly _returnvalue))

(fn InitEditor
  (bind _returnvalue (Game|GetPlayerController 0))
  (Game|Player|SetViewTargetwithBlend _returnvalue self 0.0 "VTBlend_Linear" 0.0 false)
  (Variables|/Script/Engine.PlayerController|SetbShowMouseCursor _returnvalue true)
  (Variables|/Script/Engine.PlayerController|SetbEnableClickEvents _returnvalue true)
  (Input|SetInputModeGameandUI _returnvalue 0 "DoNotLock" true))

(fn CreateEagle
  (Game|SpawnActorfromClass "/Game/Blueprints/Tile/Tile_Eagle.Tile_Eagle_C" (Math|Transform|MakeTransform (Math|Vector|MakeVector 192.0 384.0 0.0) "0, 0, 0" "1,1,1") "AlwaysSpawn" 0 0)
  (CallFunction|CreateSurrounding false))

(fn CreatePainters
  (params (StartX :type Float%20%28single-precision%29) (StartY :type Float%20%28single-precision%29) (Space :type Float%20%28single-precision%29))
  (bind _painterreturn (LocalVariables|GetPainterReturn))
  (for (_array_element _array_index) (Variables|Config|GetPainters)
    (bind _returnvalue (Game|SpawnActorfromClass _array_element (Math|Transform|MakeTransform (Math|Vector|MakeVector StartX (+ StartY (* _array_index Space)) 0.0) "0, 0, 0" "1,1,1") "AlwaysSpawn" 0 (Variables|Config|GetbEditor) 0))
    (Utilities|Array|Add _painterreturn _returnvalue))
  (return _painterreturn))

(fn LoadLevel
  (params (Level :type Integer))
  (bind _tiles (Default|LoadLevel (.AsBP%20Game%20Instance (Utilities|Casting|CastToBP_GameInstance (Game|GetGameInstance))) Level (Variables|Config|GetbEditor)))
  (if (> (Utilities|Map|Length _tiles) 0)
    (if (Variables|Config|GetbEditor)
      _
      (else
        (bind _painters (CallFunction|CreatePainters 0.0 0.0 0.0))))
    (bind _keys (Utilities|Map|Keys _tiles))
    (for _array_element _keys
      (if (Variables|Config|GetbEditor)
        (Default|CallNotifyAddTile (.Type (Utilities|Struct|BreakS_Tile (.Value (Utilities|Map|Find _tiles _array_element)))) (.Shift (Utilities|Struct|BreakS_Tile (.Value (Utilities|Map|Find _tiles _array_element)))) (Math|Vector2D|MakeVector2D (Math|Conversions|ToFloat(Integer) (/ _array_element 13)) (Math|Conversions|ToFloat(Integer) (Math|Integer|%(Integer) _array_element 13))))
        (else
          (Default|Shift (Utilities|Array|Get(acopy) _painters (.Type (Utilities|Struct|BreakS_Tile (.Value (Utilities|Map|Find _tiles _array_element))))) (* (Math|Vector|MakeVector (Math|Conversions|ToFloat(Integer) (/ _array_element 13)) (Math|Conversions|ToFloat(Integer) (Math|Integer|%(Integer) _array_element 13)) 0.0) 32.0) (.Shift (Utilities|Struct|BreakS_Tile (.Value (Utilities|Map|Find _tiles _array_element))))))))
    (for _array_element_2 _painters
      (Actor|DestroyActor _array_element_2))
    (Utilities|Array|Clear _painters)))

(fn CreateSurrounding
  (params (Shovel :type Boolean))
  (bind _returnvalue (select Shovel 16.0 8.0))
  (if (== (Utilities|Array|Length (Variables|Game|GetShovel)) 0)
    _
    (else
      (for _array_element (Variables|Game|GetShovel)
        (Actor|DestroyActor _array_element))
      (Utilities|Array|Clear (Variables|Game|GetShovel))))
  (for _array_element_2 (select Shovel (LocalVariables|GetSteelTiles) (LocalVariables|GetBrickTiles))
    (for _index (range (Math|Float|Truncate (.X (Math|Vector4|BreakVector4 _array_element_2))) (Math|Float|Truncate (.Y (Math|Vector4|BreakVector4 _array_element_2))))
      (for _index_2 (range (Math|Float|Truncate (.Z (Math|Vector4|BreakVector4 _array_element_2))) (Math|Float|Truncate (.W (Math|Vector4|BreakVector4 _array_element_2))))
        (bind _returnvalue_2 (Game|SpawnActorfromClass (select Shovel "/Game/Blueprints/Tile/Tile_Steel.Tile_Steel_C" "/Game/Blueprints/Tile/Tile_Brick.Tile_Brick_C") (Math|Transform|MakeTransform (Math|Vector|MakeVector (* _index_2 _returnvalue) (* _index _returnvalue) 0.0) "0, 0, 0" "1,1,1") "AlwaysSpawn" 0 0))
        (Utilities|Array|Add (Variables|Game|GetShovel) _returnvalue_2)))))