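; BP_ItemManager spawns power-up pickups and applies their effects in what appears to be a Battle City-style tank game.
; CreateItem places a random-type BP_Pickup on a random grid cell and binds its pickup event.
; OnPickup adds score, then dispatches by type to player buffs, the level's shovel effect, grenade damage to all enemies, or a timed enemy freeze.
; OnSpawnEnemy also freezes enemies that spawn while that timer runs.
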(event Custom|CreateItem
  (bind _returnvalue (Game|SpawnActorfromClass "/Game/Blueprints/Item/BP_Pickup.BP_Pickup_C" (Math|Transform|MakeTransform (Math|Vector|MakeVector (* (Math|Random|RandomInteger 13) 32.0) (* (Math|Random|RandomInteger 13) 32.0) 0.0) "0, 0, 0" "1,1,1") "AlwaysSpawn" 0 1e+01 0.14 (Utilities|Enum|ByteToEnumE_Item (Math|Conversions|ToByte(Integer) (Math|Random|RandomInteger 6))) 500 0))
  (EventDispatchers|BindEventtoOnPickUp _returnvalue (delegate Custom|OnPickup)))

(event Custom|OnPickup
  (params (Actor :type Actor%20Object%20Reference) (Type :type E_Item%20Enum :default "NewEnumerator2") (Score :type Integer))
  (bind _asbp_player (Utilities|Casting|CastToBP_Player Actor))
  (Default|AddScore _asbp_player Score)
  (switch Utilities|FlowControl|Switch|SwitchonE_Item Type
    (:NewEnumerator2
      (CallFunction|StartGrenade _asbp_player))
    (:NewEnumerator1
      (Default|StartInvincible _asbp_player 10.5))
    (:NewEnumerator3
      (Default|StartShovel (CallFunction|GetLevel)))
    (:NewEnumerator0
      (Default|Levelup _asbp_player))
    (:NewEnumerator4
      (Default|IncTank _asbp_player 1))
    (:NewEnumerator5
      (CallFunction|StartTimer))))

(event Custom|OnSpawnEnemy
  (params (Enemy :type BP%20Enemy%20Object%20Reference))
  (if (Variables|Game|GetOnTimer)
    (Default|Freeze Enemy)))

(event Custom|StartTimer
  (Variables|Game|SetOnTimer true)
  (Utilities|Time|SetTimerbyEvent (delegate Custom|StopTimer) 4.0)
  (bind _outactors (Actor|GetAllActorsOfClass "/Game/Blueprints/Tank/Enemy/BP_Enemy.BP_Enemy_C"))
  (for _array_element _outactors
    (Default|Freeze _array_element)))

(event Custom|StartGrenade
  (params (Player :type Actor%20Object%20Reference))
  (bind _outactors (Actor|GetAllActorsOfClass "/Game/Blueprints/Tank/Enemy/BP_Enemy.BP_Enemy_C"))
  (for _array_element _outactors
    (Game|Damage|ApplyDamage _array_element 2.0 0 Player)))

(event Custom|StopTimer
  (Variables|Game|SetOnTimer false)
  (bind _outactors (Actor|GetAllActorsOfClass "/Game/Blueprints/Tank/Enemy/BP_Enemy.BP_Enemy_C"))
  (for _array_element _outactors
    (Default|UnFreeze _array_element)))

(event EventBeginPlay)