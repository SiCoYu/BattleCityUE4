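; Enemy tank Blueprint that loads its stats from the game instance's EnemyStyles by Type and is destroyed on death.
; Non-lethal hits on multi-health types refresh the state and play a hit sound.
; The starting animation index is derived from remaining health, offset for bonus tanks.
; The Movement component starts in a fixed direction after spawning and resumes its current direction on unfreeze.
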(event EventBeginPlay
  (CallFunction|SetData (Utilities|Array|Get(acopy) (Variables|/Game/Blueprints/BP_GameInstance.BP_GameInstance_C|GetEnemyStyles (CallFunction|GetGameInstanceBP)) (Variables|Config|GetType)))
  (|CallParentFunction))

(event EventDead
  (|CallParentFunction)
  (Actor|DestroyActor))

(event Game|Damage|EventAnyDamage
  (params (Damage :type Float%20%28single-precision%29) (DamageType :type Damage%20Type%20Object%20Reference) (InstigatedBy :type Controller%20Object%20Reference) (DamageCauser :type Actor%20Object%20Reference))
  (|CallParentFunction Damage DamageType InstigatedBy DamageCauser)
  (if (and (> (Variables|Default|GetHealth) 0.0) (> (.Health (Utilities|Struct|BreakS_Tank (Variables|Default|GetData))) 1))
    (CallFunction|OnStateChange (Variables|Default|GetStateOld) (Variables|Default|GetState))
    (Audio|PlaySound2D "/Game/Assets/Audio/bullet_hit_1.bullet_hit_1" 1.0 1.0 0.0 0 0)))

(fn ConstructionScript
  (|CallParentFunction))

(fn GetAnimStart
  (return (+ (Math|Float|Truncate (* (- (Variables|Default|GetHealth) 1.0) 2.0)) (* (* (Utilities|Struct|BreakS_Tank (Variables|Default|GetData)) 2) (select (Variables|Config|GetBonus) 1 0)))))

(fn OnStateFinished
  (bind _state (CallFunction|GetState))
  (switch Utilities|FlowControl|Switch|SwitchonE_State _state
    (:NewEnumerator3
      (|CallParentFunction)
      (Default|Moveby (Variables|Default|GetMovement) "NewEnumerator2"))
    (:NewEnumerator4
      (|CallParentFunction))))

(fn UnFreeze
  (bind _movement (Variables|Default|GetMovement))
  (|CallParentFunction)
  (Default|Moveby _movement (Variables|/Game/Blueprints/Tank/Component/BP_Movement.BP_Movement_C|GetDirection _movement)))