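; Base 2D tank actor with data-driven speed, health, bullets and flipbook animations.
; A state machine (Spawning, Idle, Moving, Frozen) loads per-state tags from game config to gate damage, movement and shooting, with timers ending spawn and flickering freeze.
; Shooting fills free slots in a fixed-size bullet array, capping live bullets; zero health fires kill/death notifications and spawns an explosion.
; A separate external freeze flag also blocks movement and shooting.
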(event Custom|Dead
  (Game|SpawnActorfromClass "/Game/Blueprints/Tank/BP_Explode.BP_Explode_C" (Transformation|GetActorTransform) "AlwaysSpawn" 0 0))

(event Custom|FrozenFlicker
  (Rendering|ToggleVisibility (Variables|Default|GetSprite) false))

(event EventBeginPlay
  (CallFunction|SetState "NewEnumerator3"))

(event EventSetState
  (params (State :type E_State%20Enum :default "NewEnumerator0"))
  (bind _output_get (Variables|Config|SetStateOld (Variables|Config|GetState)))
  (bind _output_get_2 (Variables|Config|SetState State))
  (Utilities|FlowControl|Sequence
    (:then_0
      (CallFunction|OnStateChange _output_get _output_get_2))
    (:then_1
      (Default|CallNotifyStateChange _output_get _output_get_2))))

(event Game|Damage|EventAnyDamage
  (params (Damage :type Float%20%28single-precision%29) (DamageType :type Damage%20Type%20Object%20Reference) (InstigatedBy :type Controller%20Object%20Reference) (DamageCauser :type Actor%20Object%20Reference))
  (bind _self self)
  (bind _value (CallFunction|CanApplyDamage))
  (if _value
    (bind _output_get (Variables|Game|SetHealth (Math|Float|Max(Float) (- (Variables|Game|GetHealth) Damage) 0.0)))
    (if (== _output_get 0.0)
      (Default|CallNotifyKilled DamageCauser _self false)
      (Default|CallNotifyDeath _self)
      (CallFunction|Dead))))

(fn ConstructionScript)

(fn SetData
  (params (Value :type S%20Tank%20Structure))
  (bind _output_get (Variables|Config|SetData Value))
  (Variables|/Game/Blueprints/Tank/Component/BP_Movement.BP_Movement_C|SetSpeed (Variables|Default|GetMovement) (.Speed (Utilities|Struct|BreakS_Tank _output_get)))
  (Utilities|Array|Resize (Variables|Game|GetBullets) (.BulletCount (Utilities|Struct|BreakS_Tank _output_get)))
  (Variables|Game|SetHealth (Math|Conversions|ToFloat(Integer) (.Health (Utilities|Struct|BreakS_Tank _output_get)))))

(fn GetAnimStart
  (return 0))

(fn SetStateAnim
  (params (Index :type Integer))
  (bind _index (CallFunction|GetAnimStart))
  (bind _data (Variables|Config|GetData))
  (bind _animation (Utilities|Struct|BreakS_Tank _data))
  (bind _returnvalue (+ _index Index))
  (if (< _returnvalue (Utilities|Array|Length _animation))
    (Sprite|SetFlipbook (Variables|Default|GetSprite) (Utilities|Array|Get(acopy) _animation _returnvalue))))

(fn OnStateChange
  (params (Old :type E_State%20Enum :default "NewEnumerator0") (New :type E_State%20Enum :default "NewEnumerator0"))
  (bind _returnvalue (Math|Conversions|ToInteger(Byte) New))
  (Utilities|FlowControl|Sequence
    (:then_0
      (Variables|Config|SetStateTag (Utilities|Array|Get(acopy) (Utilities|Struct|BreakS_Config (Variables|/Game/Blueprints/BP_GameInstance.BP_GameInstance_C|GetConfig (CallFunction|GetGameInstanceBP))) _returnvalue)))
    (:then_1
      (switch Utilities|FlowControl|Switch|SwitchonE_State New
        (:NewEnumerator0
          (CallFunction|SetStateAnim _returnvalue :!label _label))
        (:NewEnumerator1
          (goto _label))
        (:NewEnumerator3
          (Sprite|SetFlipbook (Variables|Default|GetSprite) "/Game/Assets/Animations/Effect/Spawn.Spawn")
          (Collision|SetCollisionEnabled (Variables|Default|GetBox) "NoCollision")
          (Utilities|Time|SetTimerbyFunctionName 0 "OnStateFinished" (Utilities|Struct|BreakS_State (Variables|Config|GetStateTag)) :!label _label_2))
        (:NewEnumerator4
          (bind _returnvalue_2 (Utilities|Time|SetTimerbyFunctionName 0 "FrozenFlicker" 0.15 true))
          (Variables|Game|SetFrozenTimer _returnvalue_2)
          (goto _label_2))))))

(fn OnStateFinished
  (Utilities|FlowControl|Sequence
    (:then_0
      (switch Utilities|FlowControl|Switch|SwitchonE_State (Variables|Config|GetState)
        (:NewEnumerator3
          (Collision|SetCollisionEnabled (Variables|Default|GetBox) "QueryAndPhysics"))
        (:NewEnumerator4
          (Rendering|SetVisibility (Variables|Default|GetSprite) true false)
          (Utilities|Time|ClearandInvalidateTimerbyHandle (Variables|Game|GetFrozenTimer)))))
    (:then_1
      (CallFunction|SetState "NewEnumerator0"))))

(fn Shoot
  (bind _value (CallFunction|CanShoot))
  (if _value
    (for (_array_element _array_index) (Variables|Game|GetBullets)
      (Utilities|IsValid _array_element
        (:Is%20Not%20Valid
          (CallFunction|CreateBullet _array_index)
          (return))))))

(fn CreateBullet
  (params (Index :type Integer))
  (bind _self self)
  (bind _data (Variables|Config|GetData))
  (bind (_bulletspeed _bulletpower) (Utilities|Struct|BreakS_Tank _data))
  (bind _returnvalue (Game|SpawnActorfromClass "/Game/Blueprints/Tank/BP_Bullet.BP_Bullet_C" (Math|Transform|MakeTransform (Transformation|GetActorLocation) "0, 0, 0" "1,1,1") "AlwaysSpawn" _self (Variables|/Game/Blueprints/Tank/Component/BP_Movement.BP_Movement_C|GetDirection (Variables|Default|GetMovement)) _bulletspeed _bulletpower _self))
  (Utilities|Array|SetArrayElem (Variables|Game|GetBullets) Index _returnvalue))

(fn Freeze
  (Variables|Game|SetFrozenOutside true)
  (bind _state (CallFunction|GetState))
  (if (Utilities|Enum|Equal(Enum) _state "NewEnumerator1")
    (CallFunction|SetState "NewEnumerator0")))

(fn UnFreeze
  (Variables|Game|SetFrozenOutside false))

(fn CanApplyDamage
  (return (.CanApplyDamage (Utilities|Struct|BreakS_State (Variables|Config|GetStateTag)))))

(fn CanMove
  (return (and (Utilities|Struct|BreakS_State (Variables|Config|GetStateTag)) (not (Variables|Game|GetFrozenOutside)))))

(fn CanShoot
  (return (and (Utilities|Struct|BreakS_State (Variables|Config|GetStateTag)) (not (Variables|Game|GetFrozenOutside)))))

(fn CheckFaction
  (return false))

(fn GetState
  (return (Variables|Config|GetState)))