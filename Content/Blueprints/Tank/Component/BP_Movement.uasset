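; Movement component that drives its owning tank in four directions on a tile grid.
; MoveBy sets direction, velocity and rotation, snaps the tank's cross-axis position to 16-unit tiles, then switches its state through messages to the owner.
; Tick applies the swept offset while that state is active.
; StopBy resets the state only for the current direction, and RotateTo turns the tank without moving it.
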(event EventBeginPlay
  (bind _output_get (Variables|Game|SetTarget (Components|GetOwner)))
  (Transformation|SetActorRotation _output_get (CallFunction|GetRotationbyDirection (Variables|Game|GetDirection))))

(event EventTick
  (params (DeltaSeconds :type Float%20%28single-precision%29))
  (bind _state (Class|IBState|GetState(Message) (Components|GetOwner)))
  (if (Utilities|Enum|Equal(Enum) _state "NewEnumerator1")
    (CallFunction|MoveTarget DeltaSeconds)))

(fn Move
  (bind _direction (Variables|Game|GetDirection))
  (bind _target (Variables|Game|GetTarget))
  (Variables|Game|SetOffset (* (CallFunction|GetForwardbyDirection _direction) (Variables|Config|GetSpeed)))
  (Transformation|SetActorRotation _target (CallFunction|GetRotationbyDirection _direction))
  (CallFunction|AlignTanktoTile _target _direction))

(fn AlignTanktoTile
  (params (Tank :type Actor%20Object%20Reference) (Direction :type E_Direction%20Enum :default "NewEnumerator0"))
  (bind _returnvalue (Transformation|GetActorLocation Tank))
  (switch Utilities|FlowControl|Switch|SwitchonE_Direction Direction
    (:NewEnumerator0
      (Transformation|SetActorLocation Tank (Math|Vector|MakeVector (CallFunction|AlignTile (.x _returnvalue) -16.0 16.0) (.y _returnvalue) (.z _returnvalue)) true false :!label _label))
    (:NewEnumerator1
      (Transformation|SetActorLocation Tank (Math|Vector|MakeVector (.x _returnvalue) (CallFunction|AlignTile (.y _returnvalue) -16.0 16.0) (.z _returnvalue)) true false :!label _label_2))
    (:NewEnumerator2
      (goto _label))
    (:NewEnumerator3
      (goto _label_2))))

(fn Moveby
  (params (Direction :type E_Direction%20Enum :default "NewEnumerator0"))
  (bind _value (Class|IBState|CanMove(Message) (Variables|Game|GetTarget)))
  (if _value
    (Variables|Game|SetDirection Direction)
    (CallFunction|Move)
    (Class|IBState|SetState(Message) (Variables|Game|GetTarget) "NewEnumerator1")))

(fn Stopby
  (params (Value :type E_Direction%20Enum :default "NewEnumerator0"))
  (bind _value (Class|IBState|CanMove(Message) (Variables|Game|GetTarget)))
  (if _value
    (if (== Value (Variables|Game|GetDirection))
      (Class|IBState|SetState(Message) (Variables|Game|GetTarget) "NewEnumerator0"))))

(fn MoveTarget
  (params (Delta :type Float%20%28single-precision%29))
  (Transformation|AddActorWorldOffset (Variables|Game|GetTarget) (* (Variables|Game|GetOffset) Delta) true))

(fn Rotateto
  (params (Direction :type E_Direction%20Enum :default "NewEnumerator0"))
  (bind _output_get (Variables|Game|SetDirection Direction))
  (Transformation|SetActorRotation (Variables|Game|GetTarget) (CallFunction|GetRotationbyDirection _output_get)))