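; BF_Global is a Blueprint function library of shared helpers for a tile-based game with four-way movement.
; Direction lookups return forward vectors, with UP as negative Y, and quarter-turn rotations, while tile helpers index locations on a 32-unit grid and snap values with an offset.
; Typed getters cast to the game instance, modes and player controller (from the player pawn).
; GameOver and GetLevel go through BP_GameModeLevel.
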(fn GetForwardbyDirection
  (params (Direction :type E_Direction%20Enum :default "NewEnumerator0"))
  (return (Utilities|Select :Index Direction :NewEnumerator0 "0,-1.000000, 0" :NewEnumerator1 "1.000000,0.000000, 0" :NewEnumerator2 "0,1.000000, 0" :NewEnumerator3 "-1.000000, 0, 0" :NewEnumerator4 "0, 0, 0")))

(fn GetRotationbyDirection
  (params (Direction :type E_Direction%20Enum :default "NewEnumerator0"))
  (return (Utilities|Select :Index Direction :NewEnumerator0 "0, 0, 0" :NewEnumerator1 "0,90.000000, 0" :NewEnumerator2 "0,180.000000, 0" :NewEnumerator3 "0,270.000000, 0" :NewEnumerator4 "0, 0, 0")))

(fn GameOver
  (Default|GameOver (CallFunction|GetGameModeLevel)))

(fn GetTileIndex
  (params (Location :type Vector))
  (bind _returnvalue (/ Location 32.0))
  (return (Math|Vector2D|MakeVector2D (Math|Conversions|ToFloat(Integer) (Math|Float|Floor (.x _returnvalue))) (Math|Conversions|ToFloat(Integer) (Math|Float|Floor (.y _returnvalue))))))

(fn AlignTile
  (params (Value :type Float%20%28single-precision%29) (Offset :type Float%20%28single-precision%29) (TileWidth :type Float%20%28single-precision%29))
  (return (- (* (Math|Float|Round (/ (+ Value Offset) TileWidth)) TileWidth) Offset)))

(fn GetGameInstanceBP
  (return (.AsBP%20Game%20Instance (Utilities|Casting|CastToBP_GameInstance (Game|GetGameInstance)))))

(fn GetGameModeBP
  (return (.AsBP%20Game%20Mode (Utilities|Casting|CastToBP_GameMode (Game|GetGameMode)))))

(fn GetGameModeLevel
  (return (.AsBP%20Game%20Mode%20Level (Utilities|Casting|CastToBP_GameModeLevel (Game|GetGameMode)))))

(fn GetPlayerControllerBP
  (bind _asbp_player_controller (Utilities|Casting|CastToBP_PlayerController (Game|Player|GetPlayerPawn 0)))
  (return _asbp_player_controller))

(fn GetLevel
  (bind _asbp_game_mode_level (Utilities|Casting|CastToBP_GameModeLevel (Game|GetGameMode)))
  (return (Variables|/Game/Blueprints/BP_GameModeLevel.BP_GameModeLevel_C|GetLevel _asbp_game_mode_level)))