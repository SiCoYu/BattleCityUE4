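; Tile_Brick is a brick tile that is destroyed by any damage it receives.
; At construction, InitSprite chooses one of four brick sprites from the parity of the tile's X and Y position on an 8-unit grid.
; Neighboring tiles therefore form a repeating 2x2 sprite pattern based on where they are placed.
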(event EventBeginPlay)

(event Game|Damage|EventAnyDamage
  (params (Damage :type Float%20%28single-precision%29) (DamageType :type Damage%20Type%20Object%20Reference) (InstigatedBy :type Controller%20Object%20Reference) (DamageCauser :type Actor%20Object%20Reference))
  (Actor|DestroyActor))

(fn ConstructionScript
  (|CallParentFunction)
  (CallFunction|InitSprite))

(fn InitSprite
  (bind _returnvalue (Transformation|GetActorLocation))
  (bind _returnvalue_2 (/ _returnvalue 8.0))
  (Rendering|Components|Sprite|SetSprite (Variables|Default|GetTile) (Utilities|Select :Index (+ (* (Math|Integer|%(Integer) (Math|Float|Floor (.x _returnvalue_2)) 2) 2) (Math|Integer|%(Integer) (Math|Float|Floor (.y _returnvalue_2)) 2)) :Option%200 "/Game/Assets/Sprites/Tile/SpriteBrick0.SpriteBrick0" :Option%201 "/Game/Assets/Sprites/Tile/SpriteBrick1.SpriteBrick1" :Option%202 "/Game/Assets/Sprites/Tile/SpriteBrick2.SpriteBrick2" :Option%203 "/Game/Assets/Sprites/Tile/SpriteBrick3.SpriteBrick3")))