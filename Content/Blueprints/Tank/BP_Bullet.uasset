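; BP_Bullet is a tank projectile that flies in one of four directions, using a swept offset each tick, and is destroyed by any damage.
; Tile hits run a narrow box trace that damages overlapping targets and picks a steel or normal impact sound for player shots.
; Tags copied from the owner separate teams: differing tags take damage, enemy bullets pass through allies, and other same-tag hits send a state message.
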(event OnComponentHit(Root)
  (params (HitComponent :type Primitive%20Component%20Object%20Reference) (OtherActor :type Actor%20Object%20Reference) (OtherComp :type Primitive%20Component%20Object%20Reference) (NormalImpulse :type Vector :default "0, 0, 0") (Hit :type Hit%20Result%20Structure%20%28by%20ref%29))
  (bind _returnvalue (Transformation|GetActorLocation))
  (Utilities|Casting|CastToBP_Tile OtherActor
    (:then
      (Utilities|FlowControl|Sequence
        (:then_0
          (CallFunction|HitWall Hit)
          (Utilities|Casting|CastToBP_Player (Components|GetOwner))
          (switch Utilities|FlowControl|Switch|SwitchonE_BulletHit (Variables|Game|GetBulletHit)
            (:NewEnumerator1
              (Audio|PlaySoundatLocation "/Game/Assets/Audio/bullet_hit_1.bullet_hit_1" _returnvalue "0, 0, 0" 1.0 1.0 0.0 0 0 0))
            (:NewEnumerator2
              (Audio|PlaySoundatLocation "/Game/Assets/Audio/bullet_hit_2.bullet_hit_2" _returnvalue "0, 0, 0" 1.0 1.0 0.0 0 0 0))))
        (:then_1
          (Actor|DestroyActor))))
    (:CastFailed
      (Actor|DestroyActor))))

(event OnComponentBeginOverlap(Root)
  (params (OverlappedComponent :type Primitive%20Component%20Object%20Reference) (OtherActor :type Actor%20Object%20Reference) (OtherComp :type Primitive%20Component%20Object%20Reference) (OtherBodyIndex :type Integer) (bFromSweep :type Boolean) (SweepResult :type Hit%20Result%20Structure%20%28by%20ref%29))
  (bind _tags (Variables|Actor|GetTags))
  (bind _tags_2 (Variables|/Script/Engine.Actor|GetTags OtherActor))
  (Utilities|FlowControl|Sequence
    (:then_0
      (if (> (Utilities|Array|Length _tags_2) 0)
        (if (Utilities|Array|Identical _tags _tags_2)
          (if (>= (Utilities|Array|FindItem _tags "Enemy") 0)
            (Variables|Game|SetBulletHit "NewEnumerator0")
            (else
              (Class|IBState|SetState(Message) OtherActor "NewEnumerator4")
              (Variables|Game|SetBulletHit "NewEnumerator3")))
          (else
            (Game|Damage|ApplyDamage OtherActor (Variables|Config|GetPower) 0 (Components|GetOwner))
            (Variables|Game|SetBulletHit "NewEnumerator3")))))
    (:then_1
      (if (Utilities|Enum|NotEqual(Enum) (Variables|Game|GetBulletHit) "NewEnumerator0")
        (Actor|DestroyActor)))))

(event EventDestroyed)

(event Game|Damage|EventAnyDamage
  (params (Damage :type Float%20%28single-precision%29) (DamageType :type Damage%20Type%20Object%20Reference) (InstigatedBy :type Controller%20Object%20Reference) (DamageCauser :type Actor%20Object%20Reference))
  (Actor|DestroyActor))

(event EventTick
  (params (DeltaSeconds :type Float%20%28single-precision%29))
  (Transformation|AddActorWorldOffset (* (Variables|Game|GetOffset) DeltaSeconds) true))

(event EventBeginPlay
  (bind _returnvalue (Components|GetOwner))
  (Collision|IgnoreActorwhenMoving (Variables|Default|GetRoot) _returnvalue true)
  (Collision|IgnoreActorwhenMoving (Actor|GetComponentbyClass _returnvalue "/Script/Engine.BoxComponent") self true)
  (Utilities|Casting|CastToBP_Player (Components|GetOwner))
  (Audio|PlaySoundatLocation "/Game/Assets/Audio/bullet_shot.bullet_shot" (Transformation|GetActorLocation) "0, 0, 0" 1.0 1.0 0.0 0 0 0))

(fn ConstructionScript
  (bind _direction (Variables|Config|GetDirection))
  (Variables|Game|SetOffset (* (CallFunction|GetForwardbyDirection _direction) (Variables|Config|GetSpeed)))
  (Transformation|SetActorRotation (CallFunction|GetRotationbyDirection _direction))
  (Transformation|SetActorLocation (+ (Utilities|Select :Index _direction :NewEnumerator0 "0,-8.000000, 0" :NewEnumerator1 "8.000000, 0,0.000000" :NewEnumerator2 "0,8.000000, 0" :NewEnumerator3 "-8.000000,0.000000, 0" :NewEnumerator4 "0,8.000000, 0") (Transformation|GetActorLocation)) true false)
  (Variables|Default|SetTags (Variables|/Script/Engine.Actor|GetTags (Components|GetOwner))))

(fn HitWall
  (params (Hit :type Hit%20Result%20Structure))
  (bind (_bblockinghit _binitialoverlap _time _distance _location _impactpoint _normal) (Collision|BreakHitResult Hit))
  (bind _returnvalue (* _normal -12.0))
  (bind _returnvalue_2 (+ _location _returnvalue))
  (bind _returnvalue_3 (Class|PrimitiveComponent|CopyArrayOfMoveIgnoreActors (Variables|Default|GetRoot)))
  (bind (_outhits _returnvalue_4) (Class|KismetSystemLibrary|BoxTraceMultiforObjects _returnvalue_2 _returnvalue_2 "15.800000,2.000000,8.000000" (Transformation|GetActorRotation) (Variables|Config|GetTargetType) false _returnvalue_3 "None" true))
  (if _returnvalue_4
    (for _array_element _outhits
      (if (.bInitialOverlap (Collision|BreakHitResult _array_element))
        (Game|Damage|ApplyDamage (.HitActor (Collision|BreakHitResult _array_element)) (Variables|Config|GetPower) 0 0)
        (bind _astile_steel (Utilities|Casting|CastToTile_Steel (.HitActor (Collision|BreakHitResult _array_element))))
        (Utilities|IsValid _astile_steel
          (:Is%20Valid
            (Variables|Game|SetBulletHit "NewEnumerator1")))))
    (if (Utilities|Enum|Equal(Enum) (Variables|Game|GetBulletHit) "NewEnumerator0")
      (Variables|Game|SetBulletHit "NewEnumerator2"))))